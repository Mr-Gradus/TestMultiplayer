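; BP_NetworkGameInstance is a game instance Blueprint that handles hosting and discovery of LAN multiplayer sessions.
; CreateGame creates a LAN session, then opens Level1 as a listen server on success or prints an error on failure.
; GetGames searches for LAN sessions and prints each result's server name, player count and ping.
; It only reports found sessions and contains no join logic.
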(event `CreateGame`
  (`CreateSessionCallbackProxy.CreateSession` (`GameplayStatics.GetPlayerController` 0) 8 true
    (:`OnSuccess`
      (`GameplayStatics.OpenLevel` "Level1" true "listen"))
    (:`OnFailure`
      (`KismetSystemLibrary.PrintString` "Game creation error!!!"))))

(event `GetGames`
  (bind _results (`FindSessionsCallbackProxy.FindSessions` (`GameplayStatics.GetPlayerController` 0) 20 true)
    (:`OnSuccess`
      (for _array_element _results
        (`KismetSystemLibrary.PrintString` (`KismetStringLibrary.Concat_StrStr` "Server:" (`FindSessionsCallbackProxy.GetServerName` _array_element) "Players:" (`KismetStringLibrary.Conv_IntToString` (`FindSessionsCallbackProxy.GetCurrentPlayers` _array_element)) "/" (`KismetStringLibrary.Conv_IntToString` (`FindSessionsCallbackProxy.GetMaxPlayers` _array_element)) "Ping:" (`KismetStringLibrary.Conv_IntToString` (`FindSessionsCallbackProxy.GetPingInMs` _array_element))))))))