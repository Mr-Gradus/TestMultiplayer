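; BP_NetworkGameMode is a multiplayer game mode that assigns joining players to one of two teams.
; On PostLogin it casts to BP_MultiplayerController, adds it to Team2 if that array is smaller, otherwise Team1, and sets its TeamID.
; It then sends a name built from team number and one-based array index through ServerSetPlayerName.
; Logout is unhandled, so nothing here removes players from the team arrays.
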(event `self.K2_PostLogin`
  (params (NewPlayer :type "PlayerController Object Reference"))
  (bind _asbp_multiplayer_controller (cast `/Game/MyContent/BP/BP_MultiplayerController` NewPlayer)
    (:`then`
      (if (< (`KismetArrayLibrary.Array_Length` (`self.Team2`)) (`KismetArrayLibrary.Array_Length` (`self.Team1`)))
        (`/Game/MyContent/BP/BP_MultiplayerController.SetTeamID` _asbp_multiplayer_controller 2)
        (bind _returnvalue (`KismetArrayLibrary.Array_Add` (`self.Team2`) _asbp_multiplayer_controller))
        (set `self.PlayerIndex` _returnvalue)
        (else
          (`/Game/MyContent/BP/BP_MultiplayerController.SetTeamID` _asbp_multiplayer_controller 1)
          (bind _returnvalue_2 (`KismetArrayLibrary.Array_Add` (`self.Team1`) _asbp_multiplayer_controller))
          (set `self.PlayerIndex` _returnvalue_2)))
      (`/Game/MyContent/BP/BP_MultiplayerController.Server_SetPlayerName` _asbp_multiplayer_controller (`KismetTextLibrary.Conv_TextToString` (`|FormatText` "Team{1}_Player{2}" (`/Game/MyContent/BP/BP_MultiplayerController.TeamID` _asbp_multiplayer_controller) (+ (`self.PlayerIndex`) 1)))))
    (:`CastFailed`
      (`KismetSystemLibrary.PrintString` "Post login error"))))

(event `self.K2_OnLogout`
  (params (ExitingController :type "Controller Object Reference")))

(fn `UserConstructionScript`)