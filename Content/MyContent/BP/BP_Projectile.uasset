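; Multiplayer projectile actor that flies forward, damages player pawns on overlap and destroys itself on impact or when its lifetime timer expires.
; The server moves it each tick along its forward vector without sweep and handles sphere overlaps, ignoring the owner and other projectiles.
; Pawn hits apply damage through the BP_MultiplayerPawn health component.
; Any valid hit multicasts an explosion effect, then destroys the actor through a server event.
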(event `self.ReceiveBeginPlay`
  (`KismetSystemLibrary.K2_SetTimerDelegate` (delegate `LifeEnded`) (`self.TTL`)))

(event `LifeEnded`
  (`self.Server_LifeEnded`))

(event `Server_LifeEnded`
  (`self.K2_DestroyActor`))

(event `Server_Move`
  (params (DeltaTime :type "Float (double-precision)"))
  (`self.K2_SetActorLocation` (+ (`self.K2_GetActorLocation`) (* (`self.GetActorForwardVector`) (* DeltaTime (`self.Speed`))))))

(event `self.ReceiveTick`
  (params (DeltaSeconds :type "Float (single-precision)"))
  (if (`KismetSystemLibrary.IsServer`)
    (`self.Server_Move` DeltaSeconds)))

(event `self.SphereCollision.OnComponentBeginOverlap`
  (params (OverlappedComponent :type "PrimitiveComponent Object Reference") (OtherActor :type "Actor Object Reference") (OtherComp :type "PrimitiveComponent Object Reference") (OtherBodyIndex :type Integer) (bFromSweep :type Boolean) (SweepResult :type "HitResult Structure (by ref)"))
  (if (`KismetSystemLibrary.IsServer`)
    (`self.Server_Collision` OtherActor (`self.K2_GetActorLocation`))))

(event `Server_Collision`
  (params (`Other Actor` :type "Actor Object Reference") (Location :type "Vector Structure"))
  (if (!= `Other Actor` (`self.GetOwner`))
    (bind _asbp_multiplayer_pawn (cast `/Game/MyContent/BP/BP_MultiplayerPawn` `Other Actor`)
      (:`then`
        (`/Game/MyContent/BP/BP_HealthComponent.TakeDamage` (`/Game/MyContent/BP/BP_MultiplayerPawn.BP_HealthComponent` _asbp_multiplayer_pawn) (`self.Damage`)))
      (:`CastFailed`
        (cast `/Game/MyContent/BP/BP_Projectile` `Other Actor`
          (:`CastFailed`
            _))))
    (`self.Multicast_HitEffect` Location)
    (`self.Server_LifeEnded`)))

(event `SpawnHitEffects`
  (params (HitLocation :type "Vector Structure"))
  (`GameplayStatics.SpawnEmitterAtLocation` "/Game/StarterContent/Particles/P_Explosion.P_Explosion" HitLocation))

(event `Multicast_HitEffect`
  (params (`Hit Location` :type "Vector Structure"))
  (`self.SpawnHitEffects` `Hit Location`))

(fn `UserConstructionScript`)