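; Health component for BP_MultiplayerPawn that handles damage and death in multiplayer.
; TakeDamage forwards to a server event that subtracts from CurrentHealth without clamping, and the RepNotify prints health and updates the pawn's health bar.
; Server_Death destroys the pawn and adds the WBP_Gameover widget to the viewport from that same server-named event, though nothing in this graph calls it.
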(event `TakeDamage`
  (params (DamageValue :type "Float (double-precision)"))
  (`self.Server_TakeDamage` DamageValue))

(event `Server_TakeDamage`
  (params (DamageValue :type "Float (double-precision)"))
  (set `self.CurrentHealth` (- (`self.CurrentHealth`) DamageValue)))

(event `Server_Death`
  (bind _asbp_multiplayer_pawn (cast `/Game/MyContent/BP/BP_MultiplayerPawn` (`self.GetOwner`)))
  (`Actor.K2_DestroyActor` _asbp_multiplayer_pawn)
  (bind _returnvalue (`|CreateWidget` "/Game/MyContent/BP/WBP_Gameover.WBP_Gameover_C"))
  (`UserWidget.AddToViewport` _returnvalue 0))

(fn `OnRep_CurrentHealth`
  (`KismetSystemLibrary.PrintString` (`KismetTextLibrary.Conv_TextToString` (`|FormatText` "Health:{0}/{1}" (`self.CurrentHealth`) (`self.MaxHealth`))))
  (bind _asbp_multiplayer_pawn (cast `/Game/MyContent/BP/BP_MultiplayerPawn` (`self.GetOwner`)))
  (`/Game/MyContent/BP/BP_MultiplayerPawn.UpdateHealthBar` _asbp_multiplayer_pawn (`self.CurrentHealth`) (`self.MaxHealth`)))

(fn `OnRep_MaxHealth`)